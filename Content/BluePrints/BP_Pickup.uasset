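; BP_Pickup is an interactable pickup whose PickupType makes it a metal detector, colored key or note.
; The construction script sets mesh, material and transform per type; BeginPlay hides the red key's mesh.
; Interact grants the player the radar or key flag, or briefly shows a note widget with sound, then destroys the actor.
; With radar, the green key's Tick replays audio through a distance-scaled Delay, beeping faster as the player nears.
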(event `self.ReceiveBeginPlay`
  (switch `/Game/EN_Pickups` (`self.PickupType`)
    (:`NewEnumerator1`
      (`SceneComponent.SetVisibility` (`self.ObjectMesh`) false false))))

(event `self.ReceiveTick`
  (params (DeltaSeconds :type "Float (single-precision)"))
  (bind _asbp_first_person_character (cast `/Game/FirstPerson/Blueprints/BP_FirstPersonCharacter` (`GameplayStatics.GetPlayerCharacter` 0)))
  (switch `/Game/EN_Pickups` (`self.PickupType`)
    (:`NewEnumerator3`
      (if (`/Game/FirstPerson/Blueprints/BP_FirstPersonCharacter.HasRadar` _asbp_first_person_character)
        (`KismetSystemLibrary.Delay` (`self.Delay`))
        (bind _returnvalue (/ (`self.GetDistanceTo` _asbp_first_person_character self) 1000.0))
        (set `self.Delay` _returnvalue)
        (`AudioComponent.Play` (`self.Audio`) 0.0)
        (`KismetSystemLibrary.PrintString` (`KismetStringLibrary.Conv_DoubleToString` _returnvalue))))))

(event `/Game/BluePrints_Imported/BPI_Interact.Interact`
  (bind _asbp_first_person_character (cast `/Game/FirstPerson/Blueprints/BP_FirstPersonCharacter` (`GameplayStatics.GetPlayerCharacter` 0)))
  (switch `/Game/EN_Pickups` (`self.PickupType`)
    (:`NewEnumerator0`
      (set `/Game/FirstPerson/Blueprints/BP_FirstPersonCharacter.HasRadar` true _asbp_first_person_character)
      (`SceneComponent.SetVisibility` (`/Game/FirstPerson/Blueprints/BP_FirstPersonCharacter.MetalDetector` _asbp_first_person_character) true false))
    (:`NewEnumerator1`
      (set `/Game/FirstPerson/Blueprints/BP_FirstPersonCharacter.HasRedKey` true _asbp_first_person_character))
    (:`NewEnumerator2`
      (set `/Game/FirstPerson/Blueprints/BP_FirstPersonCharacter.HasBlueKey` true _asbp_first_person_character))
    (:`NewEnumerator3`
      (set `/Game/FirstPerson/Blueprints/BP_FirstPersonCharacter.HasGreenKey` true _asbp_first_person_character))
    (:`NewEnumerator4`
      (cast `/Game/FirstPerson/Blueprints/BP_FirstPersonCharacter` (`GameplayStatics.GetPlayerCharacter` 0))
      (bind _returnvalue (`|CreateWidget` "/Game/UserInterface/WBP_Note.WBP_Note_C"))
      (`UserWidget.AddToViewport` _returnvalue 0)
      (`GameplayStatics.PlaySound2D` "/Game/Audio/What-Is-It-Talking-About.What-Is-It-Talking-About" 1.0 1.0 0.0 null null)
      (`KismetSystemLibrary.Delay` 5.0)
      (`WidgetLayoutLibrary.RemoveAllWidgets`)))
  (`self.K2_DestroyActor`))

(event `self.Capsule.OnComponentBeginOverlap`
  (params (OverlappedComponent :type "PrimitiveComponent Object Reference") (OtherActor :type "Actor Object Reference") (OtherComp :type "PrimitiveComponent Object Reference") (OtherBodyIndex :type Integer) (bFromSweep :type Boolean) (SweepResult :type "HitResult Structure (by ref)")))

(fn `UserConstructionScript`
  (switch `/Game/EN_Pickups` (`self.PickupType`)
    (:`NewEnumerator0`
      (`StaticMeshComponent.SetStaticMesh` (`self.ObjectMesh`) "/Game/Models/SM_Metal_Detector.SM_Metal_Detector")
      (`PrimitiveComponent.SetMaterial` (`self.ObjectMesh`) 0 "/Game/Materials/M_MetalDetector.M_MetalDetector")
      (`SceneComponent.SetRelativeScale3D` (`self.ObjectMesh`) (0.125 0.125 0.125))
      (`SceneComponent.K2_SetRelativeRotation` (`self.ObjectMesh`) (struct :`Pitch` -20.0) false false))
    (:`NewEnumerator1`
      (`StaticMeshComponent.SetStaticMesh` (`self.ObjectMesh`) "/Game/Models/SM_Key.SM_Key")
      (`PrimitiveComponent.SetMaterial` (`self.ObjectMesh`) 0 "/Game/Materials/M_RedKey.M_RedKey")
      (`SceneComponent.SetRelativeScale3D` (`self.ObjectMesh`) (0.0625 0.0625 0.0625) :!label _label)
      (`SceneComponent.K2_SetRelativeRotation` :`self` (`self.ObjectMesh`) :!label _label_2))
    (:`NewEnumerator2`
      (`StaticMeshComponent.SetStaticMesh` (`self.ObjectMesh`) "/Game/Models/SM_Key.SM_Key")
      (`PrimitiveComponent.SetMaterial` (`self.ObjectMesh`) 0 "/Game/Materials/M_BlueKey.M_BlueKey")
      (goto _label))
    (:`NewEnumerator3`
      (`StaticMeshComponent.SetStaticMesh` (`self.ObjectMesh`) "/Game/Models/SM_Key.SM_Key")
      (`PrimitiveComponent.SetMaterial` (`self.ObjectMesh`) 0 "/Game/Materials/M_GreenKey.M_GreenKey")
      (goto _label))
    (:`NewEnumerator4`
      (`StaticMeshComponent.SetStaticMesh` (`self.ObjectMesh`) "/Game/Models/note.note")
      (`PrimitiveComponent.SetMaterial` (`self.ObjectMesh`) 0 "/Game/Materials/M_Note.M_Note")
      (`SceneComponent.SetRelativeScale3D` (`self.ObjectMesh`) (18.0 18.0 18.0))
      (goto _label_2))))