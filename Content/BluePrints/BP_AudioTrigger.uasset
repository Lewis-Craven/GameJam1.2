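; BP_AudioTrigger is a placeable trigger that plays a one-shot audio cue, apparently voice lines, when the player reaches it.
; The construction script maps the AudioCues selection to one of a few preset sounds on the Audio component.
; When BP_FirstPersonCharacter begins overlapping the Box, the sound plays and HasTriggered is set so it never replays.
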(event `self.Box.OnComponentBeginOverlap`
  (params (OverlappedComponent :type "PrimitiveComponent Object Reference") (OtherActor :type "Actor Object Reference") (OtherComp :type "PrimitiveComponent Object Reference") (OtherBodyIndex :type Integer) (bFromSweep :type Boolean) (SweepResult :type "HitResult Structure (by ref)"))
  (cast `/Game/FirstPerson/Blueprints/BP_FirstPersonCharacter` OtherActor)
  (if (not (`self.HasTriggered`))
    (`AudioComponent.Play` (`self.Audio`) 0.0)
    (set `self.HasTriggered` true)))

(fn `UserConstructionScript`
  (switch `/Game/BluePrints/E_AudioCues` (`self.AudioCues`)
    (:`NewEnumerator0`
      (`AudioComponent.SetSound` (`self.Audio`) "/Game/Audio/Hello-Is-Anybody-Here.Hello-Is-Anybody-Here"))
    (:`NewEnumerator1`
      (`AudioComponent.SetSound` (`self.Audio`) "/Game/Audio/What-Is-It-Talking-About.What-Is-It-Talking-About"))
    (:`NewEnumerator2`
      (`AudioComponent.SetSound` (`self.Audio`) "/Game/Audio/What-Is-That-Some-Kind-Of-Floating-Eyeball.What-Is-That-Some-Kind-Of-Floating-Eyeball"))
    (:`NewEnumerator3`
      (`AudioComponent.SetSound` (`self.Audio`) "/Game/Audio/Oh-Look-A-Metal-Detector.Oh-Look-A-Metal-Detector"))))