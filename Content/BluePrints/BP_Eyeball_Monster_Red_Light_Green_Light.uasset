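; Eyeball monster that runs a Red Light, Green Light minigame, starting shortly after BeginPlay.
; A yaw timeline plays forward for green and reversed for red, rotating Mesh through MulticastRotation.
; Each finish waits a random interval, then flips phase and recolors the point light.
; During red, a looping timer checks every player's speed, but the over-threshold branch is empty, so nobody is killed yet.
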(event `self.ReceiveBeginPlay`
  ;[1 1 1] Begins Minigame
  (`KismetSystemLibrary.Delay` 1.0)
  (`self.StartGreenLight`))

(event `MulticastRotation`
  (params (NewRotation :type "Rotator Structure"))
  ;[1 1 1] Changes Rotation of eye
  (`SceneComponent.K2_SetRelativeRotation` (`self.Mesh`) NewRotation false false))

(event `StartGreenLight`
  ;[1 1 1] Animation of eye turning
  (set `self.RedorGreenLight?` false)
  (bind (_direction _newtrack_0) (`Timeline|Timeline` :!via `PlayFromStart` :!label _label)
    (:`Update`
      (`self.MulticastRotation` (`KismetMathLibrary.MakeRotator` 0.0 0.0 _newtrack_0)))
    (:`Finished`
      (if (`self.RedorGreenLight?`)
        ;[1 1 1] Changes from red light to green light
        (bind _returnvalue (`KismetSystemLibrary.K2_SetTimerDelegate` (delegate `CheckForMovingPlayers`) 0.1 true))
        (set `self.CheckPlayerTimer` _returnvalue)
        (`KismetSystemLibrary.Delay` (`KismetMathLibrary.RandomFloatInRange` 0.5 3.0))
        (`KismetSystemLibrary.K2_ClearAndInvalidateTimerHandle` (`self.CheckPlayerTimer`))
        (`self.StartGreenLight`)
        (`KismetSystemLibrary.Delay` 0.5)
        (`LightComponent.SetLightColor` (`self.PointLight`) (struct :`G` 1.0 :`B` 0.138169 :`A` 1.0) true)
        (else
          ;[1 1 1] Changes from green light to red light
          (`KismetSystemLibrary.Delay` (`KismetMathLibrary.RandomFloatInRange` 0.5 1.5))
          (`self.StartRedLight`)
          (`KismetSystemLibrary.Delay` 0.5)
          (`LightComponent.SetLightColor` (`self.PointLight`) (struct :`R` 1.0 :`A` 1.0) true))))))

(event `StartRedLight`
  ;[1 1 1] Animation of eye turning
  (set `self.RedorGreenLight?` true)
  (goto _label :!via `ReverseFromEnd`))

(event `CheckForMovingPlayers`
  ;[1 1 1] Checks for moving players and kills if they do
  (for _array_element (`GameStateBase.PlayerArray` (`GameplayStatics.GetGameState`))
    (bind _asbp_first_person_character (cast `/Game/FirstPerson/Blueprints/BP_FirstPersonCharacter` (`PlayerState.GetPawn` _array_element)))
    (if (> (`KismetMathLibrary.VSize` (`self.GetVelocity` _asbp_first_person_character)) 10.0)
      _)))

(fn `UserConstructionScript`
  (`SceneComponent.SetVisibility` (`self.Mesh`) false false)
  (`SceneComponent.SetVisibility` (`self.EyeMonster_Mesh`) true false))