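; Blue button in a Simon Says puzzle, pressed with E after the player overlaps its box, which shows an interact popup.
; A press after the green cube is pressed beeps, brightens the material and sets BlueButtonPressed.
; An out-of-order press once the trigger's sequence completes shows game over and pauses.
; End overlap restores the HUD but never closes the gates or clears the in-range flag.
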(event `Key|E` :consume false
  (params (Key :type "Key Structure"))
  (:`Pressed`
    (if (not (`self.BlueButtonPressed`))
      (bind _returnvalue (`GameplayStatics.GetActorOfClass` "/Game/BluePrints/SimonSaysButtons/BP_GreenCube.BP_GreenCube_C"))
      (if (`/Game/BluePrints/SimonSaysButtons/BP_GreenCube.GreenButtonPressed` _returnvalue)
        (`/Engine/EditorBlueprintResources/StandardMacros.Gate` true :!label _label
          (:`Exit`
            (`Widget.RemoveFromParent` (stale `self.Box.OnComponentBeginOverlap` _returnvalue))
            (`GameplayStatics.PlaySound2D` "/Game/Sound/short-beep-tone-47916.short-beep-tone-47916" 1.0 1.0 0.0 null null)
            (`PrimitiveComponent.SetMaterial` (`self.BlueCube`) 0 "/Game/Materials/M_BrighterBlueCube.M_BrighterBlueCube")
            (set `self.BlueButtonPressed` true)))
        (else
          (bind _returnvalue_2 (`GameplayStatics.GetActorOfClass` "/Game/BluePrints/SimonSaysButtons/SimonSaysTrigger.SimonSaysTrigger_C"))
          (if (`/Game/BluePrints/SimonSaysButtons/SimonSaysTrigger.SequenceComplete` _returnvalue_2)
            (if (`self.IsInButtonRange`)
              (`Widget.RemoveFromParent` (stale `self.Box.OnComponentBeginOverlap` _returnvalue))
              (`GameplayStatics.PlaySound2D` "/Game/Sound/short-beep-tone-47916.short-beep-tone-47916" 1.0 1.0 0.0 null null)
              (`/Engine/EditorBlueprintResources/StandardMacros.Gate` true :!label _label_2
                (:`Exit`
                  (bind _returnvalue_3 (`|CreateWidget` "/Game/UserInterface/WBP_GameOver.WBP_GameOver_C"))
                  (`UserWidget.AddToViewport` _returnvalue_3 0)
                  (set `PlayerController.bShowMouseCursor` true (`GameplayStatics.GetPlayerController` 0))
                  (`GameplayStatics.SetGamePaused` true))))))))))

(event `self.Box.OnComponentBeginOverlap`
  (params (OverlappedComponent :type "PrimitiveComponent Object Reference") (OtherActor :type "Actor Object Reference") (OtherComp :type "PrimitiveComponent Object Reference") (OtherBodyIndex :type Integer) (bFromSweep :type Boolean) (SweepResult :type "HitResult Structure (by ref)"))
  (cast `/Game/FirstPerson/Blueprints/BP_FirstPersonCharacter` OtherActor)
  (bind _returnvalue (`|CreateWidget` "/Game/UserInterface/InteractPopupWidget.InteractPopupWidget_C"))
  (`UserWidget.AddToViewport` _returnvalue 0)
  (set `self.IsInButtonRange` true)
  (`|ExecutionSequence`
    (:`then_0`
      (goto _label :!via `Open`))
    (:`then_1`
      (goto _label_2 :!via `Open`))))

(event `self.Box.OnComponentEndOverlap`
  (params (OverlappedComponent :type "PrimitiveComponent Object Reference") (OtherActor :type "Actor Object Reference") (OtherComp :type "PrimitiveComponent Object Reference") (OtherBodyIndex :type Integer))
  (cast `/Game/FirstPerson/Blueprints/BP_FirstPersonCharacter` OtherActor)
  (`Widget.RemoveFromParent` (stale `self.Box.OnComponentBeginOverlap` _returnvalue))
  (`WidgetLayoutLibrary.RemoveAllWidgets`)
  (bind _returnvalue (`|CreateWidget` "/Game/UserInterface/WBP_HUD.WBP_HUD_C"))
  (`UserWidget.AddToViewport` _returnvalue 0))

(fn `UserConstructionScript`)