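; Trigger volume that plays the Simon Says demonstration sequence when the first-person character overlaps its box.
; It finds the red, green, blue and yellow cube actors by class and flashes each in that fixed order with a brighter material and a beep, using timed delays between steps.
; After the last cube reverts, it sets SequenceComplete to true.
; Nothing guards against retriggering on repeated overlaps.
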(event `self.Box.OnComponentBeginOverlap`
  (params (OverlappedComponent :type "PrimitiveComponent Object Reference") (OtherActor :type "Actor Object Reference") (OtherComp :type "PrimitiveComponent Object Reference") (OtherBodyIndex :type Integer) (bFromSweep :type Boolean) (SweepResult :type "HitResult Structure (by ref)"))
  (cast `/Game/FirstPerson/Blueprints/BP_FirstPersonCharacter` OtherActor)
  (bind _returnvalue (`GameplayStatics.GetActorOfClass` "/Game/BluePrints/SimonSaysButtons/BP_RedCube.BP_RedCube_C"))
  (`PrimitiveComponent.SetMaterial` (`StaticMeshActor.StaticMeshComponent` _returnvalue) 0 "/Game/Materials/M_BrighterRedCube.M_BrighterRedCube")
  (`GameplayStatics.PlaySound2D` "/Game/Sound/short-beep-tone-47916.short-beep-tone-47916" 1.0 1.0 0.0 null null)
  (`KismetSystemLibrary.Delay` 0.5)
  (`PrimitiveComponent.SetMaterial` (`StaticMeshActor.StaticMeshComponent` _returnvalue) 0 "/Game/Materials/M_RedCube.M_RedCube")
  (bind _returnvalue_2 (`GameplayStatics.GetActorOfClass` "/Game/BluePrints/SimonSaysButtons/BP_GreenCube.BP_GreenCube_C"))
  (`PrimitiveComponent.SetMaterial` (`/Game/BluePrints/SimonSaysButtons/BP_GreenCube.GreenCube` _returnvalue_2) 0 "/Game/Materials/M_BrighterGreenCube.M_BrighterGreenCube")
  (`GameplayStatics.PlaySound2D` "/Game/Sound/short-beep-tone-47916.short-beep-tone-47916" 1.0 1.0 0.0 null null)
  (`KismetSystemLibrary.Delay` 0.5)
  (`PrimitiveComponent.SetMaterial` (`/Game/BluePrints/SimonSaysButtons/BP_GreenCube.GreenCube` _returnvalue_2) 0 "/Game/Materials/M_GreenCube.M_GreenCube")
  (bind _returnvalue_3 (`GameplayStatics.GetActorOfClass` "/Game/BluePrints/SimonSaysButtons/BP_BlueCube.BP_BlueCube_C"))
  (`PrimitiveComponent.SetMaterial` (`/Game/BluePrints/SimonSaysButtons/BP_BlueCube.BlueCube` _returnvalue_3) 0 "/Game/Materials/M_BrighterBlueCube.M_BrighterBlueCube")
  (`GameplayStatics.PlaySound2D` "/Game/Sound/short-beep-tone-47916.short-beep-tone-47916" 1.0 1.0 0.0 null null)
  (`KismetSystemLibrary.Delay` 0.5)
  (`PrimitiveComponent.SetMaterial` (`/Game/BluePrints/SimonSaysButtons/BP_BlueCube.BlueCube` _returnvalue_3) 0 "/Game/Materials/M_BlueCube.M_BlueCube")
  (bind _returnvalue_4 (`GameplayStatics.GetActorOfClass` "/Game/BluePrints/SimonSaysButtons/BP_YellowCube.BP_YellowCube_C"))
  (`PrimitiveComponent.SetMaterial` (`/Game/BluePrints/SimonSaysButtons/BP_YellowCube.YellowCube` _returnvalue_4) 0 "/Game/Materials/M_BrighterYellowCube.M_BrighterYellowCube")
  (`GameplayStatics.PlaySound2D` "/Game/Sound/short-beep-tone-47916.short-beep-tone-47916" 1.0 1.0 0.0 null null)
  (`KismetSystemLibrary.Delay` 0.5)
  (`PrimitiveComponent.SetMaterial` (`/Game/BluePrints/SimonSaysButtons/BP_YellowCube.YellowCube` _returnvalue_4) 0 "/Game/Materials/M_YellowCube.M_YellowCube")
  (set `self.SequenceComplete` true))

(fn `UserConstructionScript`)