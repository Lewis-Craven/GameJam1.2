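; BP_RedCube is the red button cube in a Simon Says button puzzle, pressed with E.
; Box overlap by the first-person character shows an interact popup, sets the range flag and opens a gate; leaving clears all widgets and recreates the HUD, without resetting either.
; Once SimonSaysTrigger's SequenceComplete is true, E removes the popup, beeps and, through the gate, brightens the material and sets RedButtonPressed, blocking repeat presses.
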(event `Key|E` :consume false
  (params (Key :type "Key Structure"))
  (:`Pressed`
    (if (not (`self.RedButtonPressed`))
      (bind _returnvalue (`GameplayStatics.GetActorOfClass` "/Game/BluePrints/SimonSaysButtons/SimonSaysTrigger.SimonSaysTrigger_C"))
      (if (`/Game/BluePrints/SimonSaysButtons/SimonSaysTrigger.SequenceComplete` _returnvalue)
        (if (`self.Is in button range`)
          (`Widget.RemoveFromParent` (stale `self.Box.OnComponentBeginOverlap` _returnvalue))
          (`GameplayStatics.PlaySound2D` "/Game/Sound/short-beep-tone-47916.short-beep-tone-47916" 1.0 1.0 0.0 null null)
          (`/Engine/EditorBlueprintResources/StandardMacros.Gate` true :!label _label
            (:`Exit`
              (`PrimitiveComponent.SetMaterial` (`self.StaticMeshComponent`) 0 "/Game/Materials/M_BrighterRedCube.M_BrighterRedCube")
              (set `self.RedButtonPressed` true))))))))

(event `self.Box.OnComponentBeginOverlap`
  (params (OverlappedComponent :type "PrimitiveComponent Object Reference") (OtherActor :type "Actor Object Reference") (OtherComp :type "PrimitiveComponent Object Reference") (OtherBodyIndex :type Integer) (bFromSweep :type Boolean) (SweepResult :type "HitResult Structure (by ref)"))
  (cast `/Game/FirstPerson/Blueprints/BP_FirstPersonCharacter` OtherActor)
  (bind _returnvalue (`|CreateWidget` "/Game/UserInterface/InteractPopupWidget.InteractPopupWidget_C"))
  (`UserWidget.AddToViewport` _returnvalue 0)
  (set `self.Is in button range` true)
  (goto _label :!via `Open`))

(event `self.Box.OnComponentEndOverlap`
  (params (OverlappedComponent :type "PrimitiveComponent Object Reference") (OtherActor :type "Actor Object Reference") (OtherComp :type "PrimitiveComponent Object Reference") (OtherBodyIndex :type Integer))
  (cast `/Game/FirstPerson/Blueprints/BP_FirstPersonCharacter` OtherActor)
  (`Widget.RemoveFromParent` (stale `self.Box.OnComponentBeginOverlap` _returnvalue))
  (`WidgetLayoutLibrary.RemoveAllWidgets`)
  (bind _returnvalue (`|CreateWidget` "/Game/UserInterface/WBP_HUD.WBP_HUD_C"))
  (`UserWidget.AddToViewport` _returnvalue 0))

(fn `UserConstructionScript`)