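; Maze eyeball monster pawn that chases the first player's character while IsActivated is set, with its Mesh hidden at construction.
; Tick re-issues AI MoveTo at the player and runs a Delay-gated beep whose interval scales with distance, so beeps quicken as it closes in.
; When a BP_FirstPersonCharacter overlaps DeathCollision, it calls MulticastDeath on the character returned by GetActorOfClass, not necessarily the overlapping one.
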(event `self.ReceiveTick`
  (params (DeltaSeconds :type "Float (single-precision)"))
  (bind _returnvalue (`GameplayStatics.GetPlayerCharacter` 0))
  ;[1 1 1] Makes The Eyeball Monster Move Towards The Player Indefinitely
  (if (`self.IsActivated`)
    ;[1 1 1] Makes Beeps Faster The Closer It Gets To Player
    (`|ExecutionSequence`
      (:`then_0`
        (bind _asbp_first_person_character (cast `/Game/FirstPerson/Blueprints/BP_FirstPersonCharacter` (`GameplayStatics.GetPlayerCharacter` 0)))
        (`KismetSystemLibrary.Delay` (`self.BeepDelay`))
        (bind _returnvalue_2 (/ (`self.GetDistanceTo` _asbp_first_person_character self) 1000.0))
        (set `self.BeepDelay` _returnvalue_2)
        (`AudioComponent.Play` (`self.Audio`) 0.0)
        (`KismetSystemLibrary.PrintString` (`KismetStringLibrary.Conv_DoubleToString` _returnvalue_2)))
      (:`then_1`
        (cast `/Game/FirstPerson/Blueprints/BP_FirstPersonCharacter` _returnvalue)
        (`|AIMoveTo` self (1447.0 1240.0 0.0) _returnvalue)))))

(event `self.DeathCollision.OnComponentBeginOverlap`
  (params (OverlappedComponent :type "PrimitiveComponent Object Reference") (OtherActor :type "Actor Object Reference") (OtherComp :type "PrimitiveComponent Object Reference") (OtherBodyIndex :type Integer) (bFromSweep :type Boolean) (SweepResult :type "HitResult Structure (by ref)"))
  (cast `/Game/FirstPerson/Blueprints/BP_FirstPersonCharacter` OtherActor)
  (`KismetSystemLibrary.PrintString` "Hello")
  (bind _returnvalue (`GameplayStatics.GetActorOfClass` "/Game/FirstPerson/Blueprints/BP_FirstPersonCharacter.BP_FirstPersonCharacter_C"))
  (`/Game/FirstPerson/Blueprints/BP_FirstPersonCharacter.MulticastDeath` _returnvalue))

(fn `UserConstructionScript`
  (`SceneComponent.SetVisibility` (`self.Mesh`) false false))