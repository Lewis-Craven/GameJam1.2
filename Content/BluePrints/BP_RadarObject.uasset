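; Radar target actor that beeps faster as the first-person player gets closer and disappears when reached.
; While the player has the radar, Tick runs through a Delay that throttles the audio pulse, then resets the interval to player distance divided by 1000.
; Each pulse also prints that value to screen.
; A sphere overlap with the player character destroys the actor.
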(event `self.ReceiveBeginPlay`)

(event `self.ReceiveTick`
  (params (DeltaSeconds :type "Float (single-precision)"))
  ;[1 1 1] Radar System
  (bind _asbp_first_person_character (cast `/Game/FirstPerson/Blueprints/BP_FirstPersonCharacter` (`GameplayStatics.GetPlayerCharacter` 0)))
  (if (`/Game/FirstPerson/Blueprints/BP_FirstPersonCharacter.HasRadar` _asbp_first_person_character)
    (`KismetSystemLibrary.Delay` (`self.Delay`))
    (bind _returnvalue (/ (`self.GetDistanceTo` _asbp_first_person_character self) 1000.0))
    (set `self.Delay` _returnvalue)
    (`AudioComponent.Play` (`self.Audio`) 0.0)
    (`KismetSystemLibrary.PrintString` (`KismetStringLibrary.Conv_DoubleToString` _returnvalue))))

(event `self.Sphere.OnComponentBeginOverlap`
  (params (OverlappedComponent :type "PrimitiveComponent Object Reference") (OtherActor :type "Actor Object Reference") (OtherComp :type "PrimitiveComponent Object Reference") (OtherBodyIndex :type Integer) (bFromSweep :type Boolean) (SweepResult :type "HitResult Structure (by ref)"))
  (cast `/Game/FirstPerson/Blueprints/BP_FirstPersonCharacter` OtherActor)
  (`self.K2_DestroyActor`))

(fn `UserConstructionScript`)