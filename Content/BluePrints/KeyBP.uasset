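; Key pickup actor that the player collects with F, playing a sound and destroying itself.
; Overlapping component R shows a prompt widget and opens a Gate that lets the F press through.
; Leaving removes the prompt but never closes the Gate or clears the range flag, so F still works afterwards.
; A teleport to the Red Light Green Light teleport actor is left disconnected, though that actor is still looked up.
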(event `Key|F`
  (params (Key :type "Key Structure"))
  (:`Pressed`
    (if (not (`self.Has Been Picked Up`))
      (`Widget.RemoveFromParent` (stale `self.r.OnComponentBeginOverlap` _returnvalue))
      (`/Engine/EditorBlueprintResources/StandardMacros.Gate` true :!label _label
        (:`Exit`
          (`GameplayStatics.PlaySound2D` null 1.0 1.0 0.0 null null)
          (set `self.Has Been Picked Up` true)
          (bind _asbp_first_person_character (cast `/Game/FirstPerson/Blueprints/BP_FirstPersonCharacter` (`GameplayStatics.GetPlayerCharacter` 0)))
          (bind _returnvalue (`GameplayStatics.GetActorOfClass` "/Game/BluePrints/BP_PlayerTeleport_RedLightGreenLight.BP_PlayerTeleport_RedLightGreenLight_C"))
          (`self.K2_DestroyActor`))))))

(event `self.r.OnComponentBeginOverlap`
  (params (OverlappedComponent :type "PrimitiveComponent Object Reference") (OtherActor :type "Actor Object Reference") (OtherComp :type "PrimitiveComponent Object Reference") (OtherBodyIndex :type Integer) (bFromSweep :type Boolean) (SweepResult :type "HitResult Structure (by ref)"))
  (cast `/Game/FirstPerson/Blueprints/BP_FirstPersonCharacter` OtherActor)
  (if (not (`self.Has Been Picked Up`))
    (bind _returnvalue (`|CreateWidget` "/Game/UserInterface/PickupPopupWidget.PickupPopupWidget_C"))
    (`UserWidget.AddToViewport` _returnvalue 0)
    (set `self.Is In Button Range` true)
    (goto _label :!via `Open`)))

(event `self.r.OnComponentEndOverlap`
  (params (OverlappedComponent :type "PrimitiveComponent Object Reference") (OtherActor :type "Actor Object Reference") (OtherComp :type "PrimitiveComponent Object Reference") (OtherBodyIndex :type Integer))
  (cast `/Game/FirstPerson/Blueprints/BP_FirstPersonCharacter` OtherActor)
  (`Widget.RemoveFromParent` (stale `self.r.OnComponentBeginOverlap` _returnvalue)))

(fn `UserConstructionScript`)