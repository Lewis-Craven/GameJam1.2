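; BP_BigDoor is an interactable door that serves as a transition point between game areas.
; On Interact, its Teleport value selects either loading the Labyrinth level or moving the player to a destination actor if they hold the required colored key.
; Some teleports also toggle eye actors' activation.
; IsLocked sets material and collision, while the swing-open timeline and unlock logic are disconnected and never run.
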(event `self.ReceiveBeginPlay`
  ;[1 1 1] Sets The Speed of The Door Opening
  (`TimelineComponent.SetPlayRate` (`self.Door Open Timeline`) (`self.DoorOpenSpeed`))
  (if (`self.IsLocked`)
    (`PrimitiveComponent.SetCollisionEnabled` (`self.Door_CollisionBox`) "QueryAndPhysics")))

(event `self.Interact`
  (bind _asbp_first_person_character (cast `/Game/FirstPerson/Blueprints/BP_FirstPersonCharacter` (`GameplayStatics.GetPlayerCharacter` 0)))
  (`|ExecutionSequence`
    (:`then_0`
      (if (== (`self.Teleport`) 0.0)
        (`GameplayStatics.OpenLevelBySoftObjectPtr` "/Game/labyrinth.labyrinth")))
    (:`then_1`
      (if (== (`self.Teleport`) 1.0)
        (if (`/Game/FirstPerson/Blueprints/BP_FirstPersonCharacter.HasRedKey` _asbp_first_person_character)
          (bind _returnvalue (`GameplayStatics.GetActorOfClass` "/Game/BluePrints/BP_PlayerTeleport_RedLightGreenLight.BP_PlayerTeleport_RedLightGreenLight_C"))
          (`self.K2_TeleportTo` _asbp_first_person_character (`self.K2_GetActorLocation` _returnvalue) (`self.K2_GetActorRotation` _returnvalue)))))
    (:`then_2`
      (if (== (`self.Teleport`) 2.0)
        (if (`/Game/FirstPerson/Blueprints/BP_FirstPersonCharacter.HasBlueKey` _asbp_first_person_character)
          (bind _returnvalue_2 (`GameplayStatics.GetActorOfClass` "/Game/BluePrints/BP_PlayerTeleport_Labyrinth.BP_PlayerTeleport_Labyrinth_C"))
          (`self.K2_TeleportTo` _asbp_first_person_character (`self.K2_GetActorLocation` _returnvalue_2) (`self.K2_GetActorRotation` _returnvalue_2)))))
    (:`then_3`
      ;[1 1 1] Radar maze
      (if (== (`self.Teleport`) 3.0)
        (if (`/Game/FirstPerson/Blueprints/BP_FirstPersonCharacter.HasGreenKey` _asbp_first_person_character)
          (bind _returnvalue_3 (`GameplayStatics.GetActorOfClass` "/Game/BluePrints/BP_PlayerTeleport_Maze1.BP_PlayerTeleport_Maze1_C"))
          (`self.K2_TeleportTo` _asbp_first_person_character (`self.K2_GetActorLocation` _returnvalue_3) (`self.K2_GetActorRotation` _returnvalue_3))
          (set `/Game/BluePrints/BP_Eyeball_Monster_Maze.IsActivated` true (`self.EyeRef`)))))
    (:`then_4`
      (if (== (`self.Teleport`) 4.0)
        (if (`/Game/FirstPerson/Blueprints/BP_FirstPersonCharacter.HasGreenKey` _asbp_first_person_character)
          (bind _returnvalue_4 (`GameplayStatics.GetActorOfClass` "/Game/BluePrints/BP_PlayerTeleport_Maze2.BP_PlayerTeleport_Maze2_C"))
          (`self.K2_TeleportTo` _asbp_first_person_character (`self.K2_GetActorLocation` _returnvalue_4) (`self.K2_GetActorRotation` _returnvalue_4))
          (set `/Game/BluePrints/BP_Eyeball_Monster_Maze.IsActivated` true (`self.EyeRef2`)))))
    (:`then_5`
      (if (== (`self.Teleport`) 5.0)
        (if (`/Game/FirstPerson/Blueprints/BP_FirstPersonCharacter.HasGreenKey` _asbp_first_person_character)
          (bind _returnvalue_5 (`GameplayStatics.GetActorOfClass` "/Game/BluePrints/BP_PlayerTeleport_EndRoom.BP_PlayerTeleport_EndRoom_C"))
          (`self.K2_TeleportTo` _asbp_first_person_character (`self.K2_GetActorLocation` _returnvalue_5) (`self.K2_GetActorRotation` _returnvalue_5))
          (set `/Game/BluePrints/BP_Eyeball_Monster_Maze.IsActivated` false (`self.EyeRef2`)))))))

(fn `UserConstructionScript`
  (if (`self.IsLocked`)
    (`PrimitiveComponent.SetMaterial` (`self.Door`) 0 "/Game/Materials/M_ReduceHealth.M_ReduceHealth")
    (`PrimitiveComponent.SetCollisionEnabled` (`self.NPC_CollisionBox`) "QueryAndPhysics")
    (else
      (`PrimitiveComponent.SetMaterial` (`self.Door`) 0 "/Game/Materials/M_Door.M_Door")
      (`PrimitiveComponent.SetCollisionEnabled` (`self.NPC_CollisionBox`) "QueryOnly"))))