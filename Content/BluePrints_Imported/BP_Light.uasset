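; Configurable light actor whose Selection mode makes it a regular light, a flickering light, a switched light or a proximity-driven colour changer.
; The construction script shows the switch parts only for switched lights and sets a fixed colour for all modes except colour change.
; Tick toggles visibility after a delay to flicker, or lerps between two colours by player distance.
; Interact toggles switched lights, swapping the button material and playing a sound.
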(event `self.ReceiveTick`
  (params (DeltaSeconds :type "Float (single-precision)"))
  ;[1 1 1] Light Flickering
  (switch `/Game/BluePrints_Imported/ENums/ELightTypes` (`self.Selection`)
    (:`NewEnumerator1`
      (`KismetSystemLibrary.Delay` (`self.Duration`))
      (`SceneComponent.ToggleVisibility` (`self.PointLight`) false))
    (:`NewEnumerator3`
      ;[1 1 1] Lerping between two colours based on proximity to the point light
      ;;[1 1 1] Get the players and light location to determine how quickly the lerp will transition between colours
      (bind _asbp_first_person_character (cast `/Game/FirstPerson/Blueprints/BP_FirstPersonCharacter` (`GameplayStatics.GetPlayerCharacter` 0)))
      (`LightComponent.SetLightColor` (`self.PointLight`) (`KismetMathLibrary.LinearColorLerp` (`self.FarColour`) (`self.CloseColour`) (/ (`KismetMathLibrary.Vector_Distance` (`SceneComponent.K2_GetComponentLocation` (`self.PointLight`)) (`self.K2_GetActorLocation` _asbp_first_person_character)) (`self.Distance`))) true))))

(event `/Game/BluePrints_Imported/BPI_Interact.Interact`
  ;[1 1 1] Turn Light On/Off
  ;;[1 1 1] Flickering Lights Can't Turn Off Manually
  (switch `/Game/BluePrints_Imported/ENums/ELightTypes` (`self.Selection`)
    (:`NewEnumerator0`
      (if (`self.IsOn`)
        (`PrimitiveComponent.SetMaterial` (`self.Button`) 0 "/Game/Materials/M_ReduceHealth.M_ReduceHealth")
        (else
          (`PrimitiveComponent.SetMaterial` (`self.Button`) 0 "/Game/Materials/M_Door.M_Door")))
      (`SceneComponent.ToggleVisibility` (`self.PointLight`) false)
      (set `self.IsOn` (not (`self.IsOn`)))
      (`GameplayStatics.PlaySound2D` "/Game/Audio/PIXABAYlock-the-door.PIXABAYlock-the-door" 1.0 1.0 0.0 null null))))

(fn `UserConstructionScript`
  ;[1 1 1] Makes Light Switch Visible/Invisible Depending On Light Type
  (switch `/Game/BluePrints_Imported/ENums/ELightTypes` (`self.Selection`)
    (:`NewEnumerator0`
      (`SceneComponent.SetVisibility` (`self.Light Switch Casing`) true false)
      (`SceneComponent.SetVisibility` (`self.SphereCollision`) true false)
      (`SceneComponent.SetVisibility` (`self.Button`) true false)
      (`PrimitiveComponent.SetMaterial` (`self.Button`) 0 "/Game/Materials/M_Door.M_Door")
      (`LightComponent.SetLightColor` (`self.PointLight`) (`self.New Light Colour`) true))
    (:`NewEnumerator1`
      (`LightComponent.SetLightColor` (`self.PointLight`) (`self.New Light Colour`) true :!label _label)
      (`SceneComponent.SetVisibility` (`self.Light Switch Casing`) false false :!label _label_2)
      (`SceneComponent.SetVisibility` (`self.SphereCollision`) false false)
      (`SceneComponent.SetVisibility` (`self.Button`) false false))
    (:`NewEnumerator2`
      (goto _label))
    (:`NewEnumerator3`
      (goto _label_2))))