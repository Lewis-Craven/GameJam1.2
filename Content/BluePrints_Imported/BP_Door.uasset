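; BP_Door is a lockable swinging door that the player unlocks with the green key and that eyeball maze monsters open by overlap when unlocked.
; A forward-vector dot product picks the swing direction, and timelines drive the rotation for player and monster separately.
; The player timeline's update also toggles IsDoorOpen and opens the Labyrinth level.
; The construction script sets material and collision from the lock state.
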(event `self.ReceiveBeginPlay`
  ;[1 1 1] Sets The Speed of The Door Opening
  (`TimelineComponent.SetPlayRate` (`self.Door Open Timeline`) (`self.DoorOpenSpeed`))
  (if (`self.IsLocked`)
    (`PrimitiveComponent.SetCollisionEnabled` (`self.Door_CollisionBox`) "QueryAndPhysics")))

(event `/Game/BluePrints_Imported/BPI_Interact.Interact`
  ;[1 1 1] Open Door Interaction
  ;;[1 1 1] Checks If Door Is Locked
  (if (`self.IsLocked`)
    ;;[1 1 1] Unlocks The Door
    (`AudioComponent.Play` (`self.PIXABAYlock-the-door`) 0.0)
    (bind _asbp_first_person_character (cast `/Game/FirstPerson/Blueprints/BP_FirstPersonCharacter` (`GameplayStatics.GetPlayerCharacter` 0)))
    (if (`/Game/FirstPerson/Blueprints/BP_FirstPersonCharacter.HasGreenKey` _asbp_first_person_character)
      (set `self.IsLocked` false)
      (`PrimitiveComponent.SetCollisionEnabled` (`self.Door_CollisionBox`) "NoCollision")
      (`PrimitiveComponent.SetMaterial` (`self.Door`) 0 "/Game/Materials/M_Door.M_Door")
      (if (`self.IsDoorOpen`) :!label _label
        ;;[1 1 1] Gets player position to determine which side of the door they are on
        (`AudioComponent.Play` (`self.PIXABAYdoor-open-close_OPEN`) 0.0)
        (bind _asbp_first_person_character_2 (cast `/Game/FirstPerson/Blueprints/BP_FirstPersonCharacter` (`GameplayStatics.GetPlayerCharacter` 0)))
        (`/Engine/EditorBlueprintResources/StandardMacros.CompareFloat` (`KismetMathLibrary.Dot_VectorVector` (`SceneComponent.GetForwardVector` (`self.Arrow`)) (`SceneComponent.GetForwardVector` (`/Game/FirstPerson/Blueprints/BP_FirstPersonCharacter.FirstPersonCamera` _asbp_first_person_character_2)))
          (:`>`
            (set `self.RotateDirection` (struct :`Yaw` 90.0))
            ;;[1 1 1] Opens the door
            (bind (_direction _newtrack_1) (`Timeline|Door Open Timeline` :!label _label_2)
              (:`Update`
                (`SceneComponent.K2_SetRelativeRotation` (`self.Door`) (`KismetMathLibrary.RLerp` (struct) (`self.RotateDirection`) _newtrack_1) false false)
                (set `self.IsDoorOpen` (not (`self.IsDoorOpen`)))
                (`GameplayStatics.OpenLevelBySoftObjectPtr` "/Game/labyrinth.labyrinth"))))
          (:`<`
            (set `self.RotateDirection` (struct :`Yaw` -90.0))
            (goto _label_2)))
        (else
          (`AudioComponent.Play` (`self.PIXABAYdoor-open-close_CLOSE`) 0.0)
          (goto _label_2 :!via `Reverse`))))
    (else
      (goto _label))))

(event `self.NPC_CollisionBox.OnComponentBeginOverlap`
  (params (OverlappedComponent :type "PrimitiveComponent Object Reference") (OtherActor :type "Actor Object Reference") (OtherComp :type "PrimitiveComponent Object Reference") (OtherBodyIndex :type Integer) (bFromSweep :type Boolean) (SweepResult :type "HitResult Structure (by ref)"))
  ;[1 1 1] Opens The Door For NPC Using Collision Box
  (if (not (`self.IsLocked`))
    ;;[1 1 1] Gets the NPCs position  to determine which side of the door they are on
    (bind _asbp_eyeball_monster_maze (cast `/Game/BluePrints/BP_Eyeball_Monster_Maze` OtherActor))
    (`/Engine/EditorBlueprintResources/StandardMacros.CompareFloat` (`KismetMathLibrary.Dot_VectorVector` (`SceneComponent.GetForwardVector` (`self.Arrow`)) (`SceneComponent.GetForwardVector` (`Actor.RootComponent` _asbp_eyeball_monster_maze)))
      (:`>`
        (set `self.RotateDirection` (struct :`Yaw` 90.0))
        ;;[1 1 1] Same Timeline Code
        (bind (_direction _newtrack_1) (`Timeline|Timeline` :!label _label_3)
          (:`Update`
            (`SceneComponent.K2_SetRelativeRotation` (`self.Door`) (`KismetMathLibrary.RLerp` (struct) (`self.RotateDirection`) _newtrack_1) false false))))
      (:`<`
        (set `self.RotateDirection` (struct :`Yaw` -90.0))
        (goto _label_3)))))

(event `self.NPC_CollisionBox.OnComponentEndOverlap`
  (params (OverlappedComponent :type "PrimitiveComponent Object Reference") (OtherActor :type "Actor Object Reference") (OtherComp :type "PrimitiveComponent Object Reference") (OtherBodyIndex :type Integer))
  ;[1 1 1] Opens The Door For NPC Using Collision Box
  (if (not (`self.IsLocked`))
    ;;[1 1 1] Gets the NPCs position  to determine which side of the door they are on
    (cast `/Game/BluePrints/BP_Eyeball_Monster_Maze` OtherActor)
    (goto _label_3 :!via `Reverse`)))

(fn `UserConstructionScript`
  (if (`self.IsLocked`)
    (`PrimitiveComponent.SetMaterial` (`self.Door`) 0 "/Game/Materials/M_ReduceHealth.M_ReduceHealth")
    (`PrimitiveComponent.SetCollisionEnabled` (`self.NPC_CollisionBox`) "QueryAndPhysics")
    (else
      (`PrimitiveComponent.SetMaterial` (`self.Door`) 0 "/Game/Materials/M_Door.M_Door")
      (`PrimitiveComponent.SetCollisionEnabled` (`self.NPC_CollisionBox`) "QueryOnly"))))